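; Blueprint function library of global shortcuts to Game Instance services for score, foliage tree hits and a development-code flag.
; Each function gets the Game Instance, sends it the matching interface message and returns the result, so no cast to a concrete class is needed.
; The library holds no logic of its own; tree hits pass through the foliage component, hit index and health modifier.
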(fn GetAllowDevelopmentCode
  (bind _devcodeallowed (Class|BPIGameInstance|GetAllowDevelopmentCode(Message) (Game|GetGameInstance)))
  (return _devcodeallowed))

(fn GetScore
  (bind _score (Class|BPIGameInstance|GetScore(Message) (Game|GetGameInstance)))
  (return _score))

(fn IncrementScore
  (bind _score (Class|BPIGameInstance|IncrementScore(Message) (Game|GetGameInstance)))
  (return _score))

(fn OnTreeHit
  (params (Foliage%20Component :type Foliage%20Instanced%20Static%20Mesh%20Component%20Object%20Reference) (Hit%20Index :type Integer) (Health%20Modifier :type Float%20%28double-precision%29))
  (bind _status (Class|BPIGameInstance|OnTreeHit(Message) (Game|GetGameInstance) Foliage%20Component Hit%20Index Health%20Modifier))
  (return _status))