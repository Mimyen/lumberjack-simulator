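; VR game instance that holds the score and a development debug-print flag, and handles chopping of foliage trees.
; OnTreeHit keys foliage instances by component and index, starting health at 4 and applying the passed modifier.
; Each update rebuilds the health map with only that tree, discarding other trees' damage.
; At zero health, the instance is removed and three stacked, progressively rotated BP_Log actors spawn at its transform.
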(event EventInit
  (Variables|Default|SetAllowDevelopmentCode true)
  (Variables|Default|SetScore 0))

(fn PrintifAllowDevelopmentCode
  (params (Text :type String))
  (if (Variables|Default|GetAllowDevelopmentCode)
    (Development|PrintString Text))
  (return))

(fn SpawnLogs
  (params (Location :type Vector) (Rotation :type Rotator) (Scale :type Vector))
  (Game|SpawnActorfromClass "/Game/_Game/Blueprints/Objects/BP_Log.BP_Log_C" (Math|Transform|MakeTransform Location (Math|Rotator|CombineRotators Rotation "-10.000000,0.000000,0.000000") Scale) "AlwaysSpawn" "MultiplyWithRoot" 0 0)
  (Game|SpawnActorfromClass "/Game/_Game/Blueprints/Objects/BP_Log.BP_Log_C" (Math|Transform|MakeTransform (+ Location "0.000000,0.000000,103.000000") (Math|Rotator|CombineRotators Rotation "-20.000000,0.000000,0.000000") Scale) "AlwaysSpawn" "MultiplyWithRoot" 0 0)
  (Game|SpawnActorfromClass "/Game/_Game/Blueprints/Objects/BP_Log.BP_Log_C" (Math|Transform|MakeTransform (+ Location "0.000000,0.000000,206.000000") (Math|Rotator|CombineRotators Rotation "-30.000000,0.000000,0.000000") Scale) "AlwaysSpawn" "MultiplyWithRoot" 0 0))

(fn GetAllowDevelopmentCode
  (return (Variables|Default|GetAllowDevelopmentCode)))

(fn GetScore
  (return (Variables|Default|GetScore)))

(fn IncrementScore
  (bind _output_get (Variables|Default|SetScore (+ (Variables|Default|GetScore) 1)))
  (return _output_get))

(fn OnTreeHit
  (params (Foliage%20Component :type Foliage%20Instanced%20Static%20Mesh%20Component%20Object%20Reference) (Hit%20Index :type Integer) (Health%20Modifier :type Float%20%28double-precision%29))
  (bind _outinstancetransform (Components|InstancedStaticMesh|GetInstanceTransform Foliage%20Component Hit%20Index true))
  (bind _s_tree (Utilities|Struct|MakeS_Tree Hit%20Index Foliage%20Component))
  (bind (_location _rotation _scale) (Math|Transform|BreakTransform _outinstancetransform))
  (CallFunction|PrintifAllowDevelopmentCode (Utilities|String|ToString(Float) Health%20Modifier))
  (if (Utilities|Map|Contains (Variables|Default|GetFoliageHealthMap) _s_tree)
    (CallFunction|PrintifAllowDevelopmentCode "OnTreeHit > Tree object is already contained in the map")
    (else
      (Utilities|Map|Add (Variables|Default|GetFoliageHealthMap) _s_tree 4.0)
      (CallFunction|PrintifAllowDevelopmentCode "OnTreeHit > Tree object has been added to the map")))
  (if (.ReturnValue (Utilities|Map|Find (Variables|Default|GetFoliageHealthMap) _s_tree))
    (bind _output_get (Variables|Default|SetFoliageHealthMap (Utilities|Map|MakeMap _s_tree (+ (.Value (Utilities|Map|Find (Variables|Default|GetFoliageHealthMap) _s_tree)) Health%20Modifier))))
    (CallFunction|PrintifAllowDevelopmentCode (Utilities|String|ToString(Float) (.Value (Utilities|Map|Find _output_get _s_tree))))
    (if (<= (.Value (Utilities|Map|Find _output_get _s_tree)) 0.0)
      (Utilities|Map|Remove (Variables|Default|GetFoliageHealthMap) _s_tree)
      (CallFunction|SpawnLogs _location _rotation _scale)
      (bind _returnvalue (Class|InstancedStaticMeshComponent|RemoveInstance Foliage%20Component Hit%20Index))
      (CallFunction|PrintifAllowDevelopmentCode "OnTreeHit > Tree removed")
      (return _returnvalue)
      (else
        _))
    (else
      (Development|PrintString "Error > OnTreeHit > It appears that tree doesn't exist in Map<S_Tree, Float>FoliageHealthMap." true true "(R=1.000000,G=0.000000,B=0.031819,A=1.000000)" 1e+01)))
  (return false))