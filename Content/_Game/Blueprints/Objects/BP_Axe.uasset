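; BP_Axe is a grabbable axe that chops instanced foliage trees.
; When its Box overlap sweep result yields a foliage instanced mesh, it passes that component and instance index to OnTreeHit with minus one health, then plays a hit sound there.
; GrabComponentSnap turns mesh physics off on grab and back on when dropped.
; A TODO notes planned multi-hit removal and wood spawning.
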(event OnGrabbed(GrabComponentSnap)
  ;[0.15 0.15 0.15 0.5] "Snap" the Axe
  (Physics|SetSimulatePhysics (Variables|Debug|GetStaticMeshComponent) false))

(event OnDropped(GrabComponentSnap)
  ;[0.15 0.15 0.15 0.5] "Snap" the Axe
  (Physics|SetSimulatePhysics (Variables|Debug|GetStaticMeshComponent) true))

(event OnComponentBeginOverlap(Box)
  (params (OverlappedComponent :type Primitive%20Component%20Object%20Reference) (OtherActor :type Actor%20Object%20Reference) (OtherComp :type Primitive%20Component%20Object%20Reference) (OtherBodyIndex :type Integer) (bFromSweep :type Boolean) (SweepResult :type Hit%20Result%20Structure%20%28by%20ref%29))
  (bind (_bblockinghit _binitialoverlap _time _distance _location _impactpoint _normal _impactnormal _physmat _hitactor _hitcomponent _hitbonename _bonename _hititem) (Collision|BreakHitResult SweepResult))
  ;[0.15 0.15 0.15 0.5] Remove foliage on hit
  ; TODO: 4 hits to remove, then spawn wood
  (bind _asfoliage_instanced_static_mesh_component (Utilities|Casting|CastToFoliageInstancedStaticMeshComponent _hitcomponent))
  (if (CallFunction|GetAllowDevelopmentCode)
    (Development|PrintString "BP_Axe > Foliage Component has been hit" true true "(R=0.000000,G=0.660000,B=1.000000,A=1.000000)" 1e+01))
  (CallFunction|OnTreeHit _asfoliage_instanced_static_mesh_component _hititem -1.0)
  (Audio|PlaySoundatLocation "/Game/_Game/Sounds/axeHit.axeHit" _location "0, 0, 0" 1.0 1.0 0.0 0 0 0 0))

(fn ConstructionScript)