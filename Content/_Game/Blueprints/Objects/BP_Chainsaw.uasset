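; BP_Chainsaw is a grabbable chainsaw that damages foliage-instance trees while held and cutting.
; Collision box begin overlap stores the hit foliage component and instance index from the sweep result and sets IsCutting.
; Tick passes that tree to OnTreeHit with delta-time-scaled damage and switches engine and cutting audio, calling Play every frame.
; End overlap casts OverlappedComponent, the box itself rather than the other component, to foliage before clearing IsCutting.
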(event OnComponentBeginOverlap(C_CollisionBox)
  (params (OverlappedComponent :type Primitive%20Component%20Object%20Reference) (OtherActor :type Actor%20Object%20Reference) (OtherComp :type Primitive%20Component%20Object%20Reference) (OtherBodyIndex :type Integer) (bFromSweep :type Boolean) (SweepResult :type Hit%20Result%20Structure%20%28by%20ref%29))
  (bind (_bblockinghit _binitialoverlap _time _distance _location _impactpoint _normal _impactnormal _physmat _hitactor _hitcomponent _hitbonename _bonename _hititem) (Collision|BreakHitResult SweepResult))
  ;[0.15 0.15 0.15 0.5] Check if cutting
  (bind _asfoliage_instanced_static_mesh_component (Utilities|Casting|CastToFoliageInstancedStaticMeshComponent _hitcomponent))
  (if (CallFunction|GetAllowDevelopmentCode)
    (Development|PrintString "BP_Axe > Foliage Component has been hit" true true "(R=0.000000,G=0.660000,B=1.000000,A=1.000000)" 1e+01))
  (Variables|Default|SetbIsCutting true)
  (Variables|Default|SettTree (Utilities|Struct|MakeS_Tree _hititem _asfoliage_instanced_static_mesh_component)))

(event OnComponentEndOverlap(C_CollisionBox)
  (params (OverlappedComponent :type Primitive%20Component%20Object%20Reference) (OtherActor :type Actor%20Object%20Reference) (OtherComp :type Primitive%20Component%20Object%20Reference) (OtherBodyIndex :type Integer))
  ;[0.15 0.15 0.15 0.5] Update when stopped cutting
  (Utilities|Casting|CastToFoliageInstancedStaticMeshComponent OverlappedComponent)
  (Variables|Default|SetbIsCutting false))

(event OnGrabbed(C_GrabComponent)
  ;[0.15 0.15 0.15 0.5] Update when grabbed, dropped
  (Variables|Default|SetbIsGrabbed true))

(event OnDropped(C_GrabComponent)
  ;[0.15 0.15 0.15 0.5] Update when grabbed, dropped
  (Variables|Default|SetbIsGrabbed false))

(event EventTick
  (params (DeltaSeconds :type Float%20%28single-precision%29))
  (bind _ttree (Variables|Default|GettTree))
  (bind _audio_engine (Variables|Default|GetAudio_Engine))
  (bind _audio_cutting (Variables|Default|GetAudio_Cutting))
  (bind (_hitindex _foliagecomponent) (Utilities|Struct|BreakS_Tree _ttree))
  ;[0.15 0.15 0.15 0.5] Play sound, damage tree
  (if (Variables|Default|GetbIsGrabbed)
    (if (Variables|Default|GetbIsCutting)
      (CallFunction|OnTreeHit _foliagecomponent _hitindex (* DeltaSeconds 2.0))
      (Audio|Components|Audio|Stop _audio_engine)
      (Audio|Components|Audio|Play _audio_cutting 0.0)
      (else
        (Audio|Components|Audio|Stop _audio_cutting)
        (Audio|Components|Audio|Play _audio_engine 0.0)))
    (else
      (Audio|Components|Audio|Stop _audio_engine)
      (Audio|Components|Audio|Stop _audio_cutting))))

(fn ConstructionScript)