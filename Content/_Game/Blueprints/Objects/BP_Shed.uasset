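; BP_Shed is a goal area that adds to the score when a BP_Log enters its box.
; On each overlap it checks ActorArray, so a given log scores only the first time it enters.
; New logs increment the score and are added to the array, with nothing here removing them.
; Debug prints for scoring, repeat entries and other actors are gated behind a development-code check.
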(event OnComponentBeginOverlap(Box)
  (params (OverlappedComponent :type Primitive%20Component%20Object%20Reference) (OtherActor :type Actor%20Object%20Reference) (OtherComp :type Primitive%20Component%20Object%20Reference) (OtherBodyIndex :type Integer) (bFromSweep :type Boolean) (SweepResult :type Hit%20Result%20Structure%20%28by%20ref%29))
  (bind _devcodeallowed (CallFunction|GetAllowDevelopmentCode))
  ;[0.15 0.15 0.15 0.5] Add score whenever object enters SHED area
  (Utilities|Casting|CastToBP_Log OtherActor
    (:then
      (bind _iscontained (CallFunction|CheckifAlreadyContained OtherActor))
      (if (not _iscontained)
        (bind _score (CallFunction|IncrementScore))
        (CallFunction|AddActortoArray OtherActor)
        (if _devcodeallowed
          (Development|PrintString (Utilities|String|Append "Score: " (Utilities|String|ToString(Integer) _score)))
          (Development|PrintString (Utilities|String|Append (Utilities|GetDisplayName OtherActor) " entered SHED")))
        (elif _devcodeallowed
          (Development|PrintString "Object already entered SHED"))))
    (:CastFailed
      (if _devcodeallowed
        (Development|PrintString "Something else than BP_Ball entered the SHED")))))

(fn ConstructionScript)

(fn CheckifAlreadyContained
  (params (Actor :type Actor%20Object%20Reference))
  (return (Utilities|Array|ContainsItem (Variables|Default|GetActorArray) Actor)))

(fn AddActortoArray
  (params (Actor :type Actor%20Object%20Reference))
  (bind _returnvalue (Utilities|Array|Add (Variables|Default|GetActorArray) Actor))
  (return _returnvalue))