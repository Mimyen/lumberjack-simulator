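; BP_Log is a grabbable log object that plays a fall sound when it hits the landscape.
; Its grab component turns physics simulation off on the log mesh when grabbed and back on when dropped.
; A capsule overlap cast to Landscape triggers the audio, with an IsPlaying flag blocking retriggers until playback finishes.
; Debug prints for the hit and failed cast appear only when development code is allowed.
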(event OnAudioFinished(A_Log_Fall)
  ;[0.15 0.15 0.15 0.5] After finishing set isPlaying to false
  (Variables|Default|SetbIsPlaying false))

(event OnGrabbed(C_GrabComponent)
  ;[0.15 0.15 0.15 0.5] Disable physics after picking up the object
  (Physics|SetSimulatePhysics (Variables|Components|GetSM_Log3) false))

(event OnDropped(C_GrabComponent)
  ;[0.15 0.15 0.15 0.5] Disable physics after picking up the object
  (Physics|SetSimulatePhysics (Variables|Components|GetSM_Log3) true))

(event OnComponentBeginOverlap(C_Capsule)
  (params (OverlappedComponent :type Primitive%20Component%20Object%20Reference) (OtherActor :type Actor%20Object%20Reference) (OtherComp :type Primitive%20Component%20Object%20Reference) (OtherBodyIndex :type Integer) (bFromSweep :type Boolean) (SweepResult :type Hit%20Result%20Structure%20%28by%20ref%29))
  (bind _devcodeallowed (CallFunction|GetAllowDevelopmentCode))
  ;[0.15 0.15 0.15 0.5] Play sound after hitting the ground
  (Utilities|Casting|CastToLandscape OtherActor
    (:then
      (if _devcodeallowed
        (Development|PrintString "BP_Log >> Object hit the ground"))
      (if (not (Variables|Default|GetbIsPlaying))
        (Audio|Components|Audio|Play (Variables|Default|GetA_Log_Fall) 0.0)
        (Variables|Default|SetbIsPlaying true)))
    (:CastFailed
      (if _devcodeallowed
        (Development|PrintString "BP_Log >> Failed to cast other object as Landscape")))))

(fn ConstructionScript)